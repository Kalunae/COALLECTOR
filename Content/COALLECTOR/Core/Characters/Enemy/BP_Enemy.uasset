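; BP_Enemy is an enemy character with a randomized appearance and a death animation.
; Its construction script picks a random body material and gives a 30% chance of hair with a random mesh and color, drawing both colors from the same material array.
; On BeginPlay it binds to the stat component's OnDeath event, and its Die event plays the death montage on the mesh.
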(event Custom|Die
  (Animation|Montage|PlayMontage (Variables|Character|GetMesh) "/Game/COALLECTOR/Characters/Elf/Animations/AM_Death.AM_Death"))

(event EventBeginPlay
  (EventDispatchers|BindEventtoOnDeath (Variables|Default|GetBP_StatComponent) (EventDispatchers|CreateEvent :!event Custom|Die)))

(fn ConstructionScript
  (Utilities|FlowControl|Sequence ; Randomize the enemy's appearance.
    (:then_0
      ;[0 0 0] Body
      (Rendering|Material|SetMaterial (Variables|Character|GetMesh) 0 (.OutItem (Utilities|Array|Random (Variables|Default|GetMeshMaterials)))) ; Randomize the skin and clothing color.
    )
    (:then_1
      ;[0 0 0] Hair
      (if (Math|Random|RandomBoolwithWeight 0.3)
        (Components|StaticMesh|SetStaticMesh (Variables|Default|GetHair) (.OutItem (Utilities|Array|Random (Variables|Default|GetHairMesh)))) ; Randomize hair mesh.
        (Rendering|Material|SetMaterial (Variables|Default|GetHair) 0 (.OutItem (Utilities|Array|Random (Variables|Default|GetMeshMaterials)))) ; Randomize the hair color.
      ))))