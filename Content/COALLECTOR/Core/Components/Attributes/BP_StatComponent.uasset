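; Actor component that stores an owner's stats in a map keyed by type, with events for damage and healing.
; Both events route through ModifyStat, which clamps to zero and max, fires OnChange and writes back, or prints an error if the stat is missing.
; Zero health fires OnDeath without saving the new value.
; Heal can instead top up the current heart, treating each heart as three health points.
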(event Custom|TakeDamage
  (params (Amount :type Float%20%28double-precision%29))
  (bind _result (Math|Float|NegateFloat Amount)
    (:%20%20
      (CallFunction|ModifyStat "NewEnumerator0" _result))))

(event Custom|Heal
  (params (Amount :type Float%20%28double-precision%29) (bRecoverFullHeart :type Boolean))
  (if (not bRecoverFullHeart)
    (CallFunction|ModifyStat "NewEnumerator0" Amount)
    (else
      ;[0 0 0] Recover UP TO 1 heart.
      (CallFunction|ModifyStat "NewEnumerator0" (- 3.0 (Math|Float|%(Float) (CallFunction|GetCurrentHealth) 3.0))))))

(event EventBeginPlay)

(event EventTick
  (params (DeltaSeconds :type Float%20%28single-precision%29)))

(fn ModifyStat
  (params (Type :type EStat%20Enum :default "NewEnumerator0") (Amount :type Float%20%28double-precision%29))
  (bind _stats (Variables|Default|GetStats))
  (bind (_value _returnvalue) (Utilities|Map|Find _stats Type))
  (bind (_current _max _regenrate) (Utilities|Struct|BreakS_StatInfo _value))
  (bind _returnvalue_2 (+ Amount _current))
  (bind _returnvalue_3 (Math|Float|Clamp(Float) _returnvalue_2 0.0 _max))
  ;[0 0 0] Check if we can modify this stat's value.
  (if _returnvalue ; Is this stat implemented on\nthe owner?
    ;[0 0 0] Update the stat's values and dispatch the OnChange event.
    (Default|CallOnChange Type _returnvalue_3) ; Update the player's HUD.
    ;[0 0 0] Dispatch the OnDeath event if their health drops below 0.
    (if (and (Utilities|Enum|Equal(Enum) Type "NewEnumerator0") (<= _returnvalue_3 0.0)) ; Did their health drop below 0?
      (Default|CallOnDeath)
      (return)
      (else
        ;[0 0 0] Overwrite the current type's info with the updated values.
        (Utilities|Map|Add (Variables|Default|GetStats) Type (Utilities|Struct|MakeS_StatInfo _returnvalue_3 _max _regenrate)) ; Overwrite with the\nupdated one.
        (return)))
    (else
      ;[0 0 0] Modify nothing and return early since this stat isn't implemented on the owner.
      (Development|PrintText (Utilities|Text|FormatText "ERROR: {Owner} doesn't implent the {Stat} stat." (Components|GetOwner) (|GenerictoText Type)) true true "(R=1.000000,G=0.050000,B=0.050000,A=1.000000)" 5.0)
      (return))))

(fn GetMaxHealth
  (return (Utilities|Struct|BreakS_StatInfo (.Value (Utilities|Map|Find (Variables|Default|GetStats) "NewEnumerator0")))))

(fn GetCurrentHealth
  (return (Utilities|Struct|BreakS_StatInfo (.Value (Utilities|Map|Find (Variables|Default|GetStats) "NewEnumerator0")))))